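; Player controller that routes Enhanced Input move and jump actions to the player character at index 0.
; BeginPlay adds the PlayerInput mapping context to the local player's input subsystem.
; The normalized move input gives tank-style control: X moves the character along its forward vector and Y adds controller yaw.
; The jump action calls the character's Jump directly.
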(event Input|EnhancedActionEvents|EnhancedInputActionInputAction_Move
  (params (ActionValue :type Vector%202D%20Structure) (ElapsedSeconds :type Float%20%28double-precision%29) (TriggeredSeconds :type Float%20%28double-precision%29) (InputAction :type Input%20Action%20Object%20Reference :default "/Game/Inputs/InputAction_Move.InputAction_Move"))
  (bind _returnvalue (Game|GetPlayerCharacter 0))
  (bind _returnvalue_2 (Math|Vector2D|Normalize2D ActionValue))
  (:Triggered
    (Pawn|Input|AddMovementInput _returnvalue (* (.x _returnvalue_2) (Transformation|GetActorForwardVector (Game|GetPlayerCharacter 0))) 1.0 false)
    (Pawn|Input|AddControllerYawInput _returnvalue (.y _returnvalue_2))))

(event Input|EnhancedActionEvents|EnhancedInputActionInputAction_Jump
  (params (ActionValue :type Boolean) (ElapsedSeconds :type Float%20%28double-precision%29) (TriggeredSeconds :type Float%20%28double-precision%29) (InputAction :type Input%20Action%20Object%20Reference :default "/Game/Inputs/InputAction_Jump.InputAction_Jump"))
  (Character|Jump (Game|GetPlayerCharacter 0)))

(event EventBeginPlay
  (Input|AddMappingContext (PlayerController|LocalPlayerSubsystems|GetEnhancedInputLocalPlayerSubsystem) "/Game/Inputs/PlayerInput.PlayerInput" 0 "(bIgnoreAllPressedKeysUntilRelease=True,bForceImmediately=False,bNotifyUserSettings=False)"))

(event EventTick
  (params (DeltaSeconds :type Float%20%28single-precision%29)))

(fn ConstructionScript)